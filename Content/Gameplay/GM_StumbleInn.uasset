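; Game mode for Stumble Inn that runs a timed night, spawning the HUD and a second local player.
; A self-recalling Delay countdown updates the HUD clock until time runs out.
; It then shows the end screen with total money and profit, stops entrances and ends drinkers' night.
; Unlock mode swaps tables for BP_LevelUnlocks built from GameInstance data; table setup spawns it only outside classic mode.
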(event `self.ReceiveBeginPlay`
  (`self.SpawnHUD`)
  (`self.StartTimer` 30.0)
  (set `self.StartingMoney` (`/Game/Gameplay/GI_StumbleInn.Money` (cast `/Game/Gameplay/GI_StumbleInn` (`GameplayStatics.GetGameInstance`) :!pure true)))
  (`WidgetBlueprintLibrary.SetInputMode_GameOnly` (`GameplayStatics.GetPlayerController` 0))
  (`self.SetUpTables` true)
  (`self.SpawnPlayer`))

(event `StartTimer`
  (params (GameLength :type "Float (double-precision)" :default 120.0))
  (set `self.GameLength` GameLength)
  (`self.CountdownTimer`))

(event `CountdownTimer`
  (bind _returnvalue (`GameplayStatics.GetPlayerController` 0))
  (bind _gamelength (`self.GameLength`))
  (bind _money (`/Game/Gameplay/GI_StumbleInn.Money` (cast `/Game/Gameplay/GI_StumbleInn` (`GameplayStatics.GetGameInstance`) :!pure true)))
  (bind _w_hud (`/Game/TopDownBP/Blueprints/TopDownCharacter.W_HUD` (cast `/Game/TopDownBP/Blueprints/TopDownCharacter` (`GameplayStatics.GetPlayerPawn` 0) :!pure true)))
  (bind _output_get (set `self.GameTimer` (+ (`self.GameTimer`) (`GameplayStatics.GetWorldDeltaSeconds`))))
  (if (>= (`self.GameTimer`) (`self.GameLength`))
    (`/Game/UI/W_HUD.UpdateTime` _w_hud -3.0 true)
    (bind _returnvalue_2 (`|CreateWidget` "/Game/UI/W_EndGame.W_EndGame_C" null _money (- _money (`self.StartingMoney`))))
    (`UserWidget.AddToViewport` _returnvalue_2 0)
    (`WidgetBlueprintLibrary.SetInputMode_UIOnlyEx` _returnvalue _returnvalue_2)
    (set `PlayerController.bShowMouseCursor` true _returnvalue)
    (`Controller.StopMovement` _returnvalue)
    (bind _outactors (`GameplayStatics.GetAllActorsOfClass` "/Game/Blueprints/BP_Entrance.BP_Entrance_C"))
    (for _array_element _outactors
      (set `/Game/Blueprints/BP_Entrance.GameEnded` true _array_element))
    (bind _outactors_2 (`GameplayStatics.GetAllActorsOfClass` "/Game/Blueprints/BP_Drinker.BP_Drinker_C"))
    (for _array_element_2 _outactors_2
      (`/Game/Blueprints/BP_Drinker.EndOfNight` _array_element_2))
    (else
      (`/Game/UI/W_HUD.UpdateTime` _w_hud (* (/ _gamelength _gamelength) (/ _output_get _gamelength)) false)
      (`KismetSystemLibrary.Delay` (`GameplayStatics.GetWorldDeltaSeconds`))
      (`self.CountdownTimer`))))

(event `SetUpTables`
  (params (ClassicMode :type Boolean))
  (bind (_tablelocations _tableunlocked) (break `/Game/Gameplay/STRUCT_LevelUnlocks` (`/Game/Gameplay/GI_StumbleInn.Lvl_Classic` (cast `/Game/Gameplay/GI_StumbleInn` (`GameplayStatics.GetGameInstance`) :!pure true))))
  (if (not ClassicMode)
    (`|SpawnActorFromClass` "/Game/Blueprints/BP_LevelUnlocks.BP_LevelUnlocks_C" (`KismetMathLibrary.MakeTransform` (0.0 0.0 0.0)) "Undefined" "OverrideRootScale" null _tablelocations _tableunlocked false null)))

(event `EnterUnlockMode`
  (bind (_tablelocations _tableunlocked) (break `/Game/Gameplay/STRUCT_LevelUnlocks` (`/Game/Gameplay/GI_StumbleInn.Lvl_Classic` (cast `/Game/Gameplay/GI_StumbleInn` (`GameplayStatics.GetGameInstance`) :!pure true))))
  (bind _outactors (`GameplayStatics.GetAllActorsOfClass` "/Game/Blueprints/BP_Table.BP_Table_C"))
  (for _array_element _outactors
    (`self.K2_DestroyActor` _array_element))
  (`|SpawnActorFromClass` "/Game/Blueprints/BP_LevelUnlocks.BP_LevelUnlocks_C" (`KismetMathLibrary.MakeTransform` (0.0 0.0 0.0)) "Undefined" "OverrideRootScale" null _tablelocations _tableunlocked true null))

(event `SpawnPlayer`
  (bind _returnvalue (`GameplayStatics.CreatePlayer` -1))
  (bind _outactors (`GameplayStatics.GetAllActorsOfClass` "/Game/TopDownBP/Blueprints/TopDownCharacter.TopDownCharacter_C"))
  (`Controller.Possess` _returnvalue (`|GetArrayItem` _outactors 1)))

(event `SpawnHUD`
  (`/Game/TopDownBP/Blueprints/TopDownCharacter.CreateHUD` (cast `/Game/TopDownBP/Blueprints/TopDownCharacter` (`GameplayStatics.GetPlayerPawn` 0) :!pure true)))

(fn `UserConstructionScript`)