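; Tavern table actor that seats drinkers, matches served drinks to their orders and can be bought by clicking it in unlock mode.
; Drinker arrivals and departures update the count and group IDs, which ReturnSeatLocation turns into evenly rotated seat positions.
; Empty glasses appear as fanned-out runtime billboards until ClearTable removes them and zeroes drinkers' patience rate.
; Unlocking charges game-instance money, saves the flag and refreshes UI; checkout queue logic is left mostly disconnected.
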(event `SellItem`)

(event `RequeueCustomers`)

(event `ChangeNumberAtTable`
  (params (Change :type Integer) (Drinker :type "/Game/Blueprints/BP_Drinker Object Reference"))
  (if (not (`KismetArrayLibrary.Array_Contains` (`self.DrinkerArray`) Drinker))
    (bind _output_get (set `self.NumberAtTable` (+ Change (`self.NumberAtTable`))))
    (`KismetArrayLibrary.Array_Set` (`self.DrinkerArray`) (- _output_get 1) Drinker true)))

(event `AdjustSeatingPositions`
  (bind _tempgrouparray (`self.TempGroupArray`))
  (`KismetArrayLibrary.Array_Clear` (`self.TempGroupArray`))
  (for (_array_element _array_index) (`self.DrinkerArray`)
    (bind _personalgroupid (`/Game/Blueprints/BP_Drinker.PersonalGroupID` _array_element))
    (if (`KismetArrayLibrary.Array_Contains` _tempgrouparray _personalgroupid)
      (bind _unusedint (`self.FindUnusedGroupID` _tempgrouparray))
      (`KismetArrayLibrary.Array_Set` (`self.TempGroupArray`) _array_index _unusedint true)
      (else
        (`KismetArrayLibrary.Array_Set` _tempgrouparray _array_index _personalgroupid true)))
    (bind _seatlocation (`self.ReturnSeatLocation` true (`|GetArrayItem` (`self.TempGroupArray`) _array_index)))
    (`/Game/Blueprints/BP_Drinker.AdjustSeatPosition` _array_element _seatlocation)))

(event `DrinkerLeft`
  (params (Drinker :type "/Game/Blueprints/BP_Drinker Object Reference"))
  (bind _drinkerarray (`self.DrinkerArray`))
  (`KismetArrayLibrary.Array_Clear` (`self.TempDrinkerArray`))
  (`KismetArrayLibrary.Array_RemoveItem` _drinkerarray Drinker)
  (for (_array_element _array_index) _drinkerarray
    (set `/Game/Blueprints/BP_Drinker.PersonalGroupID` _array_index _array_element))
  (set `self.NumberAtTable` (`KismetArrayLibrary.Array_Length` (`self.DrinkerArray`)))
  (`self.AdjustSeatingPositions`))

(event `self.ReceiveActorOnClicked`
  (params (ButtonPressed :type "Key Structure"))
  (bind _asgi_stumble_inn (cast `/Game/Gameplay/GI_StumbleInn` (`GameplayStatics.GetGameInstance`) :!pure true))
  (bind (_tablelocations _tableunlocked) (break `/Game/Gameplay/STRUCT_LevelUnlocks` (`/Game/Gameplay/GI_StumbleInn.Lvl_Classic` _asgi_stumble_inn)))
  (if (and (`self.UnlockMode`) (!= (`self.UnlockID`) -1))
    (bind _success (`self.CheckBalanceAndUnlock`))
    (if _success
      (`KismetArrayLibrary.Array_Set` _tableunlocked (`self.UnlockID`) true true)
      (set `/Game/Gameplay/GI_StumbleInn.Lvl_Classic` (make `/Game/Gameplay/STRUCT_LevelUnlocks` _tablelocations _tableunlocked) _asgi_stumble_inn)
      (set `self.UnlockID` -1)
      (`PrimitiveComponent.SetMaterial` (`self.Table`) 0 "/Engine/BasicShapes/BasicShapeMaterial.BasicShapeMaterial")
      (`/Game/TopDownBP/Blueprints/TopDownController.RefreshUnlockWidget` (cast `/Game/TopDownBP/Blueprints/TopDownController` (`GameplayStatics.GetPlayerController` 0) :!pure true)))))

(event `AddEmptyGlass`
  (params (DrinkID :type Integer))
  (bind _emptyglassarray (`self.EmptyGlassArray`))
  (bind _returnvalue (`KismetArrayLibrary.Array_Length` (`self.EmptyGlassArray`)))
  (bind _returnvalue_2 (`AddComponent|NODE_AddBillboardComponent-0` :`RelativeTransform` (`KismetMathLibrary.MakeTransform` (+ (`KismetMathLibrary.GreaterGreater_VectorRotator` (`KismetMathLibrary.MakeVector` (+ (.x (`SceneComponent.GetForwardVector` (`self.Table`))) (* _returnvalue (- (`self.EmptyGlassDistanceCentre`) (/ (`KismetMathLibrary.Conv_IntToDouble` _returnvalue) 2.0)))) (.y (`SceneComponent.GetForwardVector` (`self.Table`))) (.z (`SceneComponent.GetForwardVector` (`self.Table`)))) (`KismetMathLibrary.MakeRotator` 0.0 0.0 (* _returnvalue (- (`self.EmptyGlassRotation`) (* (`KismetMathLibrary.Conv_IntToDouble` _returnvalue) 1.5))))) (0.0 0.0 110.0)))))
  (`BillboardComponent.SetSprite` _returnvalue_2 (select `int` DrinkID :`0` "/Engine/EditorResources/S_Actor.S_Actor" :`1` "/Engine/EngineResources/AICON-Red.AICON-Red" :!type "Texture2D Object Reference"))
  (`SceneComponent.SetHiddenInGame` _returnvalue_2 false false)
  (`KismetArrayLibrary.Array_Set` _emptyglassarray (`KismetArrayLibrary.Array_Length` _emptyglassarray) _returnvalue_2 true))

(event `ClearTable`
  (for _array_element (`self.EmptyGlassArray`)
    (`ActorComponent.K2_DestroyComponent` _array_element))
  (`KismetArrayLibrary.Array_Clear` (`self.EmptyGlassArray`))
  (for _array_element_2 (`self.DrinkerArray`)
    (`/Game/Blueprints/BP_Drinker.SetPatienceRate` _array_element_2 0)))

(fn `CheckBalanceAndUnlock`
  (returns (Success :type Boolean))
  (bind _unlockcost (`self.UnlockCost`))
  (bind _asgi_stumble_inn (cast `/Game/Gameplay/GI_StumbleInn` (`GameplayStatics.GetGameInstance`) :!pure true))
  (bind _money (`/Game/Gameplay/GI_StumbleInn.Money` _asgi_stumble_inn))
  (if (>= _money _unlockcost)
    (set `/Game/Gameplay/GI_StumbleInn.Money` (- _money _unlockcost) _asgi_stumble_inn)
    (`/Game/UI/W_HUD.UpdateBalance` (`/Game/TopDownBP/Blueprints/TopDownCharacter.W_HUD` (cast `/Game/TopDownBP/Blueprints/TopDownCharacter` (`GameplayStatics.GetPlayerPawn` 0) :!pure true)))
    (bind _returnvalue (`|CreateWidget` "/Game/UI/W_MoneyIndicator.W_MoneyIndicator_C" null (* (`self.UnlockCost`) -1)))
    (`UserWidget.AddToViewport` _returnvalue 0)
    (`UserWidget.SetPositionInViewport` _returnvalue (`GameplayStatics.ProjectWorldToScreen` (`GameplayStatics.GetPlayerController` 0) (`self.K2_GetActorLocation`)) true)
    (`UserWidget.SetAlignmentInViewport` _returnvalue (0.5 0.5))
    (return true)
    (else
      (return false))))

(fn `CheckCustomerOrder`
  (params (DrinkID :type Integer))
  (returns (Success :type Boolean))
  (for _array_element (`self.DrinkerArray`)
    (if (== (`/Game/Blueprints/BP_Drinker.WantedItem` _array_element) DrinkID)
      (`/Game/Blueprints/BP_Drinker.ReceiveDrink` _array_element)
      (return true)))
  (return false))

(fn `FindUnusedGroupID`
  (params (TempGroupArray :type "Array of Integer"))
  (returns (UnusedInt :type Integer))
  (for _array_element (`|MakeArray` 0 1 2 3)
    (if (not (`KismetArrayLibrary.Array_Contains` TempGroupArray _array_element))
      (return _array_element))))

(fn `PlaceItemOnCheckout`
  (params (ItemID :type Integer) (Customer :type "/Game/Blueprints/BP_Customer Object Reference") (Requeue :type Boolean))
  (returns (FirstInQueue :type Boolean))
  (set `self.ReadyToCheckout` true)
  (if (not Requeue)
    (`KismetArrayLibrary.Array_Set` (`self.CustomerArray`) (`self.NumberAtTable`) Customer true)
    (set `self.NumberAtTable` (+ (`self.NumberAtTable`) 1)))
  (switch `int` ItemID
    (:`0`
      (`SceneComponent.SetVisibility` (`self.Item`) true false)
      (return (== (`KismetArrayLibrary.Array_Find` (`self.CustomerArray`) Customer) 0)))))

(fn `ReturnSeatLocation`
  (params (Reseat :type Boolean) (PersonalGroupID :type Integer))
  (returns (SeatLocation :type "Vector Structure"))
  (locals (TempPersonalGroupID :type "Float (double-precision)"))
  (set `local.TempPersonalGroupID` (`KismetMathLibrary.Conv_IntToDouble` PersonalGroupID))
  (if Reseat
    (return (+ (`self.K2_GetActorLocation`) (* (`KismetMathLibrary.GreaterGreater_VectorRotator` (`KismetMathLibrary.GetForwardVector` (`self.K2_GetActorRotation`)) (`KismetMathLibrary.MakeRotator` 0.0 0.0 (* (/ 360.0 (`KismetMathLibrary.Conv_IntToDouble` (`self.NumberAtTable`))) (`local.TempPersonalGroupID`)))) (`self.DistanceFromTable`))))
    (else
      (return (+ (`self.K2_GetActorLocation`) (* (`KismetMathLibrary.GreaterGreater_VectorRotator` (`KismetMathLibrary.GetForwardVector` (`self.K2_GetActorRotation`)) (`KismetMathLibrary.MakeRotator` 0.0 0.0 (* (/ 720.0 (+ (`KismetMathLibrary.Conv_IntToDouble` (`self.NumberAtTable`)) 1.0)) (`local.TempPersonalGroupID`)))) (`self.DistanceFromTable`)))))))

(fn `UserConstructionScript`)