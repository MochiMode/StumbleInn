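; BP_Shelf is a shelf actor that holds one item, apparently a drink, which the player can pick up.
; StockShelf records the item ID and shows the matching placeholder-looking sprite, while the construction script hides it when unstocked.
; EmptyShelf clears the shelf only if the requested ID matches and reports success.
; PlayerPickUp empties it and returns the stored ID and sprite.
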(event `StockShelf`
  (params (ItemID :type Integer))
  (bind _item (`self.Item`))
  (set `self.Stocked` true)
  (bind _output_get (set `self.StockedItemID` ItemID))
  (switch `int` _output_get
    (:`0`
      (`BillboardComponent.SetSprite` _item "/Engine/EditorResources/S_Actor.S_Actor"))
    (:`1`
      (`BillboardComponent.SetSprite` _item "/Engine/EngineResources/AICON-Red.AICON-Red")))
  (`SceneComponent.SetVisibility` _item true false))

(fn `EmptyShelf`
  (params (WantedItemID :type Integer))
  (returns (Success :type Boolean))
  (if (== WantedItemID (`self.StockedItemID`))
    (set `self.Stocked` false)
    (set `self.StockedItemID` -1)
    (`SceneComponent.SetVisibility` (`self.Item`) false false)
    (return true)
    (else
      (return false))))

(fn `PlayerPickUp`
  (returns (DrinkID :type Integer) (Sprite :type "Texture2D Object Reference"))
  (locals (TempDrinkID :type Integer))
  (bind _output_get (set `local.TempDrinkID` (`self.StockedItemID`)))
  (`self.EmptyShelf` _output_get)
  (return _output_get (`BillboardComponent.Sprite` (`self.Item`))))

(fn `UserConstructionScript`
  (if (not (`self.Stocked`))
    (`SceneComponent.SetVisibility` (`self.Item`) false false)))