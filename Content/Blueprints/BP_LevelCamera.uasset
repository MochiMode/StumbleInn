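; BP_LevelCamera is a level camera that automatically zooms out to fit the level's static meshes in view.
; On BeginPlay it becomes the player's view target if IsActiveCamera is set, then starts the fit check.
; CheckLevelInView uses WasRecentlyRendered on every StaticMeshActor; upon finding one unseen, it lengthens the spring arm, widens the ortho width, breaks the loop, and re-runs itself after a frame-length delay.
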(event `CheckLevelInView`
  (bind _camera (`self.Camera`))
  (bind _springarm (`self.SpringArm`))
  (bind _outactors (`GameplayStatics.GetAllActorsOfClass` "/Script/Engine.StaticMeshActor"))
  (for _array_element _outactors :!label _label
    (if (not (`self.WasRecentlyRendered` _array_element 0.2))
      (set `SpringArmComponent.TargetArmLength` (+ (`SpringArmComponent.TargetArmLength` _springarm) 100.0) _springarm)
      (`CameraComponent.SetOrthoWidth` _camera (+ (`CameraComponent.OrthoWidth` _camera) 32.0))
      (`self.BreakVisionLoop`)
      (`KismetSystemLibrary.Delay` (`GameplayStatics.GetWorldDeltaSeconds`))
      (`self.CheckLevelInView`))))

(event `BreakVisionLoop`
  (goto _label :!via `Break`))

(event `self.ReceiveBeginPlay`
  (`self.SetActiveCamera`)
  (`self.CheckLevelInView`))

(event `SetActiveCamera`
  (if (`self.IsActiveCamera`)
    (`PlayerController.SetViewTargetWithBlend` (`GameplayStatics.GetPlayerController` 0) self 0.0 "VTBlend_Linear" 0.0 false)))

(fn `UserConstructionScript`)