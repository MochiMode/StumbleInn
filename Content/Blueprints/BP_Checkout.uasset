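; Shop checkout actor that queues customers, displays their item and completes a sale.
; PlaceItemOnCheckout registers new customers, marks checkout ready, and for item ID 0 shows the item and returns whether that customer is first.
; SellItem hides the item, sends the front customer to the exit, then shifts the queue array forward.
; Remaining customers move to positions spaced from QueueAnchor along the actor's rotation.
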(event `SellItem`
  (if (`self.ReadyToCheckout`)
    (`SceneComponent.SetVisibility` (`self.Item`) false false)
    (`/Game/Blueprints/BP_Customer.MoveToExit` (`|GetArrayItem` (`self.CustomerArray`)))
    (set `self.ReadyToCheckout` false)
    (`self.RequeueCustomers`)))

(event `RequeueCustomers`
  (bind _customerarray (`self.CustomerArray`))
  (`KismetArrayLibrary.Array_Clear` (`self.TempCustomerArray`))
  (for _index (range 1 (+ (`KismetArrayLibrary.Array_LastIndex` _customerarray) 1))
    (`KismetArrayLibrary.Array_Set` (`self.TempCustomerArray`) (`KismetMathLibrary.Clamp` (- _index 1) 0 999) (`|GetArrayItem` _customerarray _index) true))
  (bind _output_get (set `self.CustomerArray` (`self.TempCustomerArray`)))
  (set `self.NumberInQueue` (`KismetArrayLibrary.Array_LastIndex` _output_get))
  (for (_array_element _array_index) _output_get
    (bind _queuelocation (`self.ReturnQueueLocation` true _array_index))
    (`/Game/Blueprints/BP_Customer.MoveToRequeue` _array_element _queuelocation self)))

(fn `PlaceItemOnCheckout`
  (params (ItemID :type Integer) (Customer :type "/Game/Blueprints/BP_Customer Object Reference") (Requeue :type Boolean))
  (returns (FirstInQueue :type Boolean))
  (set `self.ReadyToCheckout` true)
  (if (not Requeue)
    (`KismetArrayLibrary.Array_Set` (`self.CustomerArray`) (`self.NumberInQueue`) Customer true)
    (set `self.NumberInQueue` (+ (`self.NumberInQueue`) 1)))
  (switch `int` ItemID
    (:`0`
      (`SceneComponent.SetVisibility` (`self.Item`) true false)
      (return (== (`KismetArrayLibrary.Array_Find` (`self.CustomerArray`) Customer) 0)))))

(fn `ReturnQueueLocation`
  (params (Requeue :type Boolean) (RequeueNumber :type Integer))
  (returns (QueueLocation :type "Vector Structure"))
  (if Requeue
    (return (+ (`SceneComponent.K2_GetComponentLocation` (`self.QueueAnchor`)) (`KismetMathLibrary.GreaterGreater_VectorRotator` (* (`self.QueueSpace`) RequeueNumber) (`self.K2_GetActorRotation`))))
    (else
      (return (+ (`SceneComponent.K2_GetComponentLocation` (`self.QueueAnchor`)) (`KismetMathLibrary.GreaterGreater_VectorRotator` (* (`self.QueueSpace`) (`self.NumberInQueue`)) (`self.K2_GetActorRotation`)))))))

(fn `UserConstructionScript`)