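; Shop customer character that finds its wanted item on a shelf, carries it to a checkout queue and can leave through the entrance.
; A gated, frame-delayed loop polls shelves for the item, then AI MoveTo steps chain through pickup, a randomly chosen checkout and item placement, retrying on failed moves.
; MoveToRequeue and MoveToExit have no callers here; they redirect the customer to a new queue spot or walk it out and destroy it.
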(event `self.ReceiveBeginPlay`
  (`self.LookForItem`))

(event `LookForItem`
  (`|ExecutionSequence`
    (:`then_0`
      (goto _label_2 :!via `Open`))
    (:`then_1`
      (bind _outactors (`GameplayStatics.GetAllActorsOfClass` "/Game/Blueprints/BP_Shelf.BP_Shelf_C"))
      (for _array_element _outactors :!label _label
        (if (== (`/Game/Blueprints/BP_Shelf.StockedItemID` _array_element) (`self.WantedItem`))
          (`self.MoveToItem` _array_element)
          (`self.BreakLookLoop`)))
      (`/Engine/EditorBlueprintResources/StandardMacros.Gate` false :!label _label_2
        (:`Exit`
          (`KismetSystemLibrary.Delay` (`GameplayStatics.GetWorldDeltaSeconds`))
          (`self.LookForItem`))))))

(event `BreakLookLoop`
  (`|ExecutionSequence`
    (:`then_0`
      (goto _label_2 :!via `Close`))
    (:`then_1`
      (goto _label :!via `Break`))))

(event `MoveToItem`
  (params (Shelf :type "/Game/Blueprints/BP_Shelf Object Reference"))
  (`|AIMoveTo` self (0.0 0.0 0.0) Shelf 150.0
    (:`OnSuccess`
      (bind _success (`/Game/Blueprints/BP_Shelf.EmptyShelf` Shelf (`self.WantedItem`)))
      (if _success
        (`self.PickupItem`)
        (else
          (`self.LookForItem`))))
    (:`OnFail`
      (`self.LookForItem`))))

(event `PickupItem`
  (`self.MoveToQueue`)
  (switch `int` (`self.WantedItem`)
    (:`0`
      (`SceneComponent.SetVisibility` (`self.Item`) true false))))

(event `MoveToQueue`
  (bind _output (`|GetArrayItem` (`self.TempCheckoutArray`)))
  (bind _outactors (`GameplayStatics.GetAllActorsOfClass` "/Game/Blueprints/BP_Checkout.BP_Checkout_C"))
  (bind _output_get (set `self.TempCheckoutArray` _outactors))
  (`KismetArrayLibrary.Array_Shuffle` _output_get)
  (bind _queuelocation (`/Game/Blueprints/BP_Checkout.ReturnQueueLocation` _output false 0))
  (`|AIMoveTo` self _queuelocation
    (:`OnSuccess`
      (bind _firstinqueue (`/Game/Blueprints/BP_Checkout.PlaceItemOnCheckout` _output (`self.WantedItem`) self false))
      (if _firstinqueue
        (`SceneComponent.SetVisibility` (`self.Item`) false false)))
    (:`OnFail`
      (`self.MoveToQueue`))))

(event `MoveToExit`
  (bind _outactors (`GameplayStatics.GetAllActorsOfClass` "/Game/Blueprints/BP_Entrance.BP_Entrance_C"))
  (`|AIMoveTo` self (0.0 0.0 0.0) (`|GetArrayItem` _outactors) 100.0
    (:`OnSuccess`
      (`self.K2_DestroyActor`))
    (:`OnFail`
      (`self.MoveToExit`))))

(event `RequeueOnFail`
  (`|AIMoveTo` self (`self.RequeueLocation`) :!label _label_3
    (:`OnSuccess`
      (bind _firstinqueue (`/Game/Blueprints/BP_Checkout.PlaceItemOnCheckout` (`self.RequeueCheckout`) (`self.WantedItem`) self true))
      (if _firstinqueue
        (`SceneComponent.SetVisibility` (`self.Item`) false false)))
    (:`OnFail`
      (`self.RequeueOnFail`))))

(event `MoveToRequeue`
  (params (Location :type "Vector Structure") (Checkout :type "/Game/Blueprints/BP_Checkout Object Reference"))
  (set `self.RequeueLocation` Location)
  (set `self.RequeueCheckout` Checkout)
  (`MovementComponent.StopMovementImmediately` (`self.CharacterMovement`))
  (goto _label_3))

(fn `UserConstructionScript`)