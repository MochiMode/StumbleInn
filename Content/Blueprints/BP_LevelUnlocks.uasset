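; BP_LevelUnlocks spawns the level's BP_Table actors at preset locations based on which tables are unlocked.
; In unlock mode it spawns every table with its index as UnlockID, then clears the ID on owned tables and gives locked ones the upgrade-available material.
; Otherwise it destroys all existing tables and spawns plain tables only at unlocked locations.
; All of this runs once on BeginPlay, driven by parallel arrays sharing one index.
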(event `self.ReceiveBeginPlay`
  (if (`self.UnlockMode`)
    (for (_array_element _array_index) (`self.TableLocations`)
      (bind _returnvalue (`|SpawnActorFromClass` "/Game/Blueprints/BP_Table.BP_Table_C" (`KismetMathLibrary.MakeTransform` _array_element) "Undefined" "OverrideRootScale" null true _array_index null))
      (`KismetArrayLibrary.Array_Set` (`self.TableArray`) _array_index _returnvalue true))
    (for (_array_element_2 _array_index_2) (`self.TableArray`)
      (if (`|GetArrayItem` (`self.TableUnlocked`) _array_index_2)
        (set `/Game/Blueprints/BP_Table.UnlockID` -1 _array_element_2)
        (else
          (`PrimitiveComponent.SetMaterial` (`/Game/Blueprints/BP_Table.Table` _array_element_2) 0 "/Game/Materials/M_Upgrade_Available.M_Upgrade_Available"))))
    (else
      (`self.RemoveExistingTables`)
      (for (_array_element_3 _array_index_3) (`self.TableUnlocked`)
        (if _array_element_3
          (`|SpawnActorFromClass` "/Game/Blueprints/BP_Table.BP_Table_C" (`KismetMathLibrary.MakeTransform` (`|GetArrayItem` (`self.TableLocations`) _array_index_3)) "Undefined" "OverrideRootScale" null false -1 null))))))

(event `RemoveExistingTables`
  (bind _outactors (`GameplayStatics.GetAllActorsOfClass` "/Game/Blueprints/BP_Table.BP_Table_C"))
  (for _array_element _outactors
    (`self.K2_DestroyActor` _array_element)))

(fn `UserConstructionScript`)