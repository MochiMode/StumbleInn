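; BP_Drinker is an inn customer that finds a table, orders one of two drinks, pays, then reorders or leaves.
; It line-traces to random tables and exits, retrying until clear, moves with AIMoveTo, and destroys itself if the table is full.
; A Patience timeline tints the speech bubble, scales tips and triggers leaving, running faster when empty glasses clutter the table.
; Unreachable shelf and checkout logic remains in the graph.
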(event Custom|LookForTable
  (bind _outactors (Actor|GetAllActorsOfClass "/Game/Blueprints/BP_Table.BP_Table_C"))
  (bind _output_get (Variables|Default|SetTempTableArray _outactors))
  (Utilities|Array|Shuffle _output_get)
  (bind _output_get_2 (Variables|Default|SetChosenTable (Utilities|Array|Get(acopy) (Variables|Default|GetTempTableArray))))
  (bind _ignoredactors (CallFunction|GetIgnoredActors false))
  (bind (_outhit _returnvalue) (Collision|LineTraceByChannel (Transformation|GetActorLocation self) (Transformation|GetActorLocation (Variables|Default|GetChosenTable)) "TraceTypeQuery1" false _ignoredactors "None"))
  (if _returnvalue
    (Utilities|Casting|CastToBP_Table (.HitActor (Collision|BreakHitResult _outhit))
      (:then
        (if (> (Variables|/Game/Blueprints/BP_Table.BP_Table_C|GetNumberAtTable _output_get_2) 2)
          (Actor|DestroyActor)
          (else
            (if (== (Variables|Default|GetPersonalGroupID) -1)
              (Variables|Default|SetPersonalGroupID (Variables|/Game/Blueprints/BP_Table.BP_Table_C|GetNumberAtTable _output_get_2))
              (Default|ChangeNumberatTable (Variables|Default|GetChosenTable) 1 self))
            (CallFunction|MovetoSeat))))
      (:CastFailed
        (Utilities|FlowControl|Delay (Utilities|Time|GetWorldDeltaSeconds) :!label _label)
        (CallFunction|LookforTable)))
    (else
      (goto _label))))

(event Custom|MoveToSeat
  (bind _seatlocation (Default|ReturnSeatLocation (Variables|Default|GetChosenTable) false (Variables|Default|GetPersonalGroupID)))
  (AI|AIMoveTo self _seatlocation 0 3e+02 false
    (:OnSuccess
      (CallFunction|SetPatienceRate (Utilities|Array|Length (Variables|/Game/Blueprints/BP_Table.BP_Table_C|GetEmptyGlassArray (Variables|Default|GetChosenTable))))
      (Default|AdjustSeatingPositions (Variables|Default|GetChosenTable))
      (CallFunction|DecideDrink))
    (:OnFail
      (CallFunction|MovetoSeat))))

(event Custom|HideWants
  (Rendering|SetVisibility (Variables|Default|GetSpeechSprite) false true))

(event Custom|MoveToExit
  (bind _outactors (Actor|GetAllActorsOfClass "/Game/Blueprints/BP_Entrance.BP_Entrance_C"))
  (bind _output_get (Variables|Default|SetTempDoorArray _outactors))
  (Utilities|Array|Shuffle _output_get)
  (bind _ignoredactors (CallFunction|GetIgnoredActors true))
  (bind (_outhit _returnvalue) (Collision|LineTraceByChannel (Transformation|GetActorLocation self) (+ (Transformation|GetWorldLocation (Variables|/Game/Blueprints/BP_Entrance.BP_Entrance_C|GetDoors (Utilities|Array|Get(acopy) (Variables|Default|GetTempDoorArray)))) "0, 0,50.000000") "TraceTypeQuery1" false _ignoredactors "None"))
  (if _returnvalue
    (Utilities|FlowControl|Delay (Utilities|Time|GetWorldDeltaSeconds))
    (CallFunction|MovetoExit)
    (else
      (AI|AIMoveTo self "0, 0, 0" (Utilities|Array|Get(acopy) (Variables|Default|GetTempDoorArray)) 1e+02 false
        (:OnSuccess
          (Actor|DestroyActor))
        (:OnFail
          (CallFunction|MovetoExit))))))

(event Custom|AdjustSeatPosition
  (params (SeatPosition :type Vector))
  (Variables|Default|SetTempSeatPosition SeatPosition)
  (AI|AIMoveTo self (Variables|Default|GetTempSeatPosition) 0 2e+01 false
    (:OnSuccess
      (if (and (Variables|Default|GetWantsDrink) (== (Variables|Default|GetWantedItem) -1))
        (CallFunction|DecideDrink)
        (CallFunction|SetPatienceRate (Utilities|Array|Length (Variables|/Game/Blueprints/BP_Table.BP_Table_C|GetEmptyGlassArray (Variables|Default|GetChosenTable))))))
    (:OnFail
      (CallFunction|MoveonAdjustFail))))

(event Custom|DrinkDrink
  (Utilities|FlowControl|Delay (Math|Random|RandomFloatinRange 4.0 12.0))
  (Default|AddEmptyGlass (Variables|Default|GetChosenTable) (Variables|Default|GetHeldDrinkID))
  (Rendering|SetVisibility (Variables|Default|GetItem) false false)
  (switch int (Math|Random|RandomInteger 2)
    (:0
      (CallFunction|DecideDrink))
    (:1
      (CallFunction|MovetoExit)
      (Default|DrinkerLeft (Variables|Default|GetChosenTable) self))))

(event Custom|EndOfNight
  (CallFunction|HideWants)
  (CallFunction|MovetoExit))

(event Custom|MoveOnAdjustFail
  (AI|AIMoveTo self (Variables|Default|GetTempSeatPosition) 0 2e+01 false
    (:OnSuccess
      (if (and (Variables|Default|GetWantsDrink) (== (Variables|Default|GetWantedItem) -1))
        (CallFunction|DecideDrink)
        (CallFunction|SetPatienceRate (Utilities|Array|Length (Variables|/Game/Blueprints/BP_Table.BP_Table_C|GetEmptyGlassArray (Variables|Default|GetChosenTable))))))
    (:OnFail
      (CallFunction|MoveonAdjustFail))))

(event Custom|MoveToRequeue
  (params (Location :type Vector) (Checkout :type BP%20Checkout%20Object%20Reference)))

(event Custom|PayForDrink
  (params (DrinkID :type Integer))
  (bind _returnvalue (Game|GetGameInstance))
  (bind _returnvalue_2 (Utilities|Select :Index DrinkID :Option%200 5.0 :Option%201 1e+01))
  (bind _patiencescore (Variables|Default|GetPatienceScore))
  (bind _returnvalue_3 (* 20 _patiencescore))
  (bind _asgi_stumble_inn (Utilities|Casting|CastToGI_StumbleInn _returnvalue))
  (bind _returnvalue_4 (UserInterface|CreateWidget "/Game/UI/W_MoneyIndicator.W_MoneyIndicator_C" 0 (Math|Float|Truncate _returnvalue_2) (Math|Float|Truncate _returnvalue_3)))
  (UserInterface|Viewport|AddtoViewport _returnvalue_4 0)
  (Class|UserWidget|SetPositioninViewport _returnvalue_4 (.ScreenPosition (Class|GameplayStatics|ProjectWorldtoScreen (Game|GetPlayerController 0) (Transformation|GetWorldLocation (Variables|Default|GetSpeechSprite)) false)) true)
  (Class|UserWidget|SetAlignmentinViewport _returnvalue_4 "(X=0.500000,Y=0.500000)")
  (Variables|/Game/Gameplay/GI_StumbleInn.GI_StumbleInn_C|SetMoney _asgi_stumble_inn (+ (Variables|/Game/Gameplay/GI_StumbleInn.GI_StumbleInn_C|GetMoney _asgi_stumble_inn) (Math|Float|Truncate (+ _returnvalue_3 _returnvalue_2))))
  (Default|UpdateBalance (Variables|/Game/TopDownBP/Blueprints/TopDownCharacter.TopDownCharacter_C|GetW_HUD (.AsTop%20Down%20Character (Utilities|Casting|CastToTopDownCharacter (Game|Player|GetPlayerPawn 0))))))

(event Custom|SetSpeechBubbleAngle
  (Transformation|SetWorldRotation (Variables|Default|GetSpeechSprite) "0.000000,90.000000,-35.000000" false false))

(event Custom|RequeueOnFail)

(event Custom|DecideDrink
  (bind _wanteddrink (Variables|Default|GetWantedDrink))
  (Variables|Default|SetWantsDrink true)
  (CallFunction|SetSpeechBubbleAngle)
  (CallFunction|StartPatienceTimer)
  (bind _output_get (Variables|Default|SetWantedItem (Math|Random|RandomInteger 2)))
  (Rendering|SetVisibility (Variables|Default|GetSpeech) true true)
  (switch int _output_get
    (:0
      (Rendering|Components|Sprite|SetSprite _wanteddrink "/Engine/EditorResources/S_Actor.S_Actor"))
    (:1
      (Rendering|Components|Sprite|SetSprite _wanteddrink "/Engine/EngineResources/AICON-Red.AICON-Red"))))

(event Custom|ReceiveDrink
  (bind _item (Variables|Default|GetItem))
  (Variables|Default|SetWantsDrink false)
  (Rendering|SetVisibility (Variables|Default|GetSpeech) false true)
  (Utilities|FlowControl|Sequence
    (:then_0
      (Rendering|SetVisibility (Variables|Default|GetItem) true false)
      (CallFunction|PayforDrink (Variables|Default|GetWantedItem))
      (CallFunction|DrinkDrink)
      (switch int (Variables|Default|GetWantedItem)
        (:0
          (Rendering|Components|Sprite|SetSprite _item "/Engine/EditorResources/S_Actor.S_Actor"))
        (:1
          (Rendering|Components|Sprite|SetSprite _item "/Engine/EngineResources/AICON-Red.AICON-Red"))))
    (:then_1
      (Variables|Default|SetHeldDrinkID (Variables|Default|GetWantedItem)))
    (:then_2
      (Variables|Default|SetWantedItem -1))))

(event Custom|BreakLookLoop
  (Utilities|FlowControl|Sequence
    (:then_0
      (Utilities|FlowControl|Gate false) ; enters at Close
    )
    (:then_1
      (Utilities|Array|ForEachLoopwithBreak (stale _outactors)) ; enters at Break
    )))

(event Custom|StartPatienceTimer
  (Utilities|FlowControl|Sequence
    (:then_0
      (bind _patience (Timeline|Patience Stop)
        (:Update
          (Variables|Default|SetPatienceScore _patience)
          (Sprite|SetSpriteColor (Variables|Default|GetSpeechSprite) (Math|Color|Lerp(LinearColor) (Variables|Default|GetColour_PatientRed) (Variables|Default|GetColour_PatientGreen) _patience)))
        (:Finished
          (if (Variables|Default|GetWantsDrink)
            (Rendering|SetVisibility (Variables|Default|GetSpeechSprite) false true)
            (CallFunction|MovetoExit)
            (Default|DrinkerLeft (Variables|Default|GetChosenTable) self)))))
    (:then_1
      (Timeline|Patience PlayFromStart))))

(event Custom|SetPatienceRate
  (params (NumberOfEmptyGlasses :type Integer))
  (Components|Timeline|SetPlayRate (Variables|Default|GetPatience) (+ (* NumberOfEmptyGlasses 0.125) 1.0)))

(event EventBeginPlay
  (CallFunction|LookforTable))

(event Collision|EventActorBeginOverlap
  (params (OtherActor :type Actor%20Object%20Reference)))

(event EventTick
  (params (DeltaSeconds :type Float%20%28single-precision%29))
  (if (Variables|Default|GetWantsDrink)
    (CallFunction|SetSpeechBubbleAngle)))

(fn ConstructionScript)

(fn GetIgnoredActors
  (params (IgnoreTables :type Boolean))
  (LocalVariables|SetLocalIgnoreTables IgnoreTables)
  (bind _outactors (Actor|GetAllActorsOfClass "/Game/TopDownBP/Blueprints/TopDownCharacter.TopDownCharacter_C"))
  (LocalVariables|SetActorArray _outactors)
  (bind _outactors_2 (Actor|GetAllActorsOfClass "BP_Drinker_C"))
  (Utilities|Array|AppendArray (LocalVariables|GetActorArray) _outactors_2)
  (if (LocalVariables|GetLocalIgnoreTables)
    (bind _outactors_3 (Actor|GetAllActorsOfClass "/Game/Blueprints/BP_Table.BP_Table_C"))
    (Utilities|Array|AppendArray (LocalVariables|GetActorArray) _outactors_3)
    (return (LocalVariables|GetActorArray))
    (else
      (return (LocalVariables|GetActorArray)))))