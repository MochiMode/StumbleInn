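; BP_Entrance is the customer entrance, spawning BP_Drinker actors at its own transform while tables have room.
; From BeginPlay it loops on a random delay between the min and max spawn delays, stopping once GameEnded is set.
; Each pass scans all BP_Table actors and spawns one drinker at the first with NumberAtTable of two or fewer, then breaks the loop.
; The group ID increment is disconnected and never runs.
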(event `self.ReceiveBeginPlay`
  (`self.RandomDelayThenCheckEmptyTables`))

(event `SpawnCustomer`
  (`|SpawnActorFromClass` "/Game/Blueprints/BP_Drinker.BP_Drinker_C" (`self.GetTransform`) "AdjustIfPossibleButAlwaysSpawn" "OverrideRootScale" null -1 null))

(event `RandomDelayThenCheckEmptyTables`
  (`KismetSystemLibrary.Delay` (`KismetMathLibrary.RandomFloatInRange` (`self.MinCustomerSpawnDelay`) (`self.MaxCustomerSpawnDelay`)))
  (if (not (`self.GameEnded`))
    (`self.CheckForEmptyTables`)))

(event `CheckForEmptyTables`
  (bind _outactors (`GameplayStatics.GetAllActorsOfClass` "/Game/Blueprints/BP_Table.BP_Table_C"))
  (for _array_element _outactors :!label _label
    (if (<= (`/Game/Blueprints/BP_Table.NumberAtTable` _array_element) 2)
      (`self.SpawnCustomer`)
      (`self.BreakEmptyTableLoop`)))
  (`self.RandomDelayThenCheckEmptyTables`))

(event `BreakEmptyTableLoop`
  (goto _label :!via `Break`))

(fn `UserConstructionScript`)